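; BP_SnakeController is the controller for the Snake game that sets up the UI and moves the game from menu to play.
; On BeginPlay it shows the main menu and score label widgets and binds to the game mode's state-change event.
; StartGame hides the menu and sets the game mode's state to Game.
; The state handler only prints a debug message for Main Menu, Game and Outro.
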(event `self.ReceiveBeginPlay`
  (bind _returnvalue (`|CreateWidget` "/Game/UI/WBP_MainMenu.WBP_MainMenu_C"))
  (bind _output_get (set `self.MainMenuRef` _returnvalue))
  (`UserWidget.AddToViewport` _output_get 0)
  (bind _returnvalue_2 (`|CreateWidget` "/Game/UI/WBP_ScoreLabel.WBP_ScoreLabel_C"))
  (`UserWidget.AddToViewport` _returnvalue_2 0)
  (bind _asbp_snake_game_mode (cast `/Game/Snake/BP_SnakeGameMode` (`GameplayStatics.GetGameMode`)))
  (add `SnakeGameMode.OnGameStateChanged` _asbp_snake_game_mode (delegate `HandleGameState`)))

(event `HandleGameState`
  (params (NewState :type "ESnakeGameState Enum" :default "MainMenu"))
  (switch `ESnakeGameState` NewState
    (:`MainMenu`
      (`KismetSystemLibrary.PrintString` "Main Menu State"))
    (:`Game`
      (`KismetSystemLibrary.PrintString` "Game State"))
    (:`Outro`
      (`KismetSystemLibrary.PrintString` "Outro State"))))

(event `StartGame`
  (`Widget.SetVisibility` (`self.MainMenuRef`) "Hidden")
  (bind _assnake_game_mode (cast `SnakeGameMode` (`GameplayStatics.GetGameMode`)))
  (`SnakeGameMode.SetGameState` _assnake_game_mode "Game"))

(fn `UserConstructionScript`)