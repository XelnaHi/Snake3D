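; BP_SnakeController is the snake game's player controller, managing per-player score UI and the game-over screen.
; After a short delay on BeginPlay, it enables pawn movement and creates a score label seeded from the player's game instance data.
; ShowOutro freezes every snake, shows the winner's game-over widget and resets game instance data.
; StartGame and ShowMainMenu toggle menu widgets, though MainMenuRef is never assigned here.
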(event `self.ReceiveBeginPlay`
  (bind _returnvalue (`self.K2_GetPawn`))
  (`KismetSystemLibrary.Delay` 0.2)
  (bind _assnake_game_instance (cast `SnakeGameInstance` (`GameplayStatics.GetGameInstance`)))
  (set `self.SGInstance` _assnake_game_instance)
  (bind _assnake_character (cast `SnakeCharacter` _returnvalue))
  (set `self.PlayerID` (`GameplayStatics.GetPlayerControllerID` (`PlayerState.GetPlayerController` (`Controller.PlayerState` (`Pawn.GetController` _returnvalue)))))
  (set `SnakeCharacter.bCanMove` true _assnake_character)
  (bind _asbp_snake_state (cast `/Game/Snake/Character/BP_SnakeState` (`Pawn.PlayerState` (`self.K2_GetPawn`))))
  (bind _returnvalue_2 (`|CreateWidget` "/Game/Snake/UI/WBP_ScoreLabel.WBP_ScoreLabel_C" self _asbp_snake_state))
  (bind _output_get (set `self.ScoreLabelRef` _returnvalue_2))
  (`UserWidget.AddToPlayerScreen` _output_get 0)
  (bind _returnvalue_3 (`SnakeGameInstance.GetSnakePlayerData` (`self.SGInstance`) (`self.PlayerID`)))
  (`/Game/Snake/UI/WBP_ScoreLabel.SetScore` (`self.ScoreLabelRef`) (`KismetMathLibrary.Conv_IntToDouble` (break `PlayerPersistentData` _returnvalue_3))))

(event `StartGame`
  ;[0.01307 0.1337 0] Start Game
  (`Widget.SetVisibility` (`self.MainMenuRef`) "Hidden")
  (bind _returnvalue (`|CreateWidget` "/Game/Snake/UI/WBP_ScoreLabel.WBP_ScoreLabel_C" null null))
  (bind _output_get (set `self.ScoreLabelRef` _returnvalue))
  (`Widget.SetVisibility` _output_get "Visible")
  (`UserWidget.AddToViewport` _output_get 0))

(event `ShowOutro`
  (params (PlayerID :type Integer))
  ;[0.07868 0.01472 0.15 0.9304] Show Outro
  (bind _outactors (`GameplayStatics.GetAllActorsOfClass` "/Game/Snake/Character/BP_SnakeCharacter_New.BP_SnakeCharacter_New_C"))
  (for _array_element _outactors
    (set `SnakeCharacter.bCanMove` false _array_element))
  (bind _returnvalue (`|CreateWidget` "/Game/Snake/UI/WBP_GameOverMenu.WBP_GameOverMenu_C" null PlayerID))
  (bind _output_get (set `self.GameOverRef` _returnvalue))
  (`UserWidget.AddToViewport` _output_get 0)
  (bind _asbp_snake_game_instance (cast `/Game/Snake/Character/BP_SnakeGameInstance` (`GameplayStatics.GetGameInstance`)))
  (`SnakeGameInstance.ResetSnakeGameInstanceData` _asbp_snake_game_instance))

(event `ShowMainMenu`
  ;[0.15 0.1079 0] Show Main Menu
  (`Widget.SetVisibility` (`self.GameOverRef`) "Hidden")
  (`Widget.SetVisibility` (`self.ScoreLabelRef`) "Visible")
  (`Widget.SetVisibility` (`self.MainMenuRef`) "Visible"))

(fn `UserConstructionScript`)