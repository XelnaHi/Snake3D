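; Snake tail actor that ends a two-player match when a snake character runs into it.
; On overlap, it identifies the colliding player by controller ID and reads the other player's score from SnakeGameInstance.
; It then calls ShowOutro on the colliding snake's controller with that opposing player's number and score.
; The tail's owner is not checked, so any player-controlled snake triggers it.
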(event `self.ReceiveActorBeginOverlap`
  (params (OtherActor :type "Actor Object Reference"))
  (bind _asbp_snake_character_new (cast `/Game/Snake/Character/BP_SnakeCharacter_New` OtherActor))
  (bind _returnvalue (`Pawn.GetController` _asbp_snake_character_new))
  (bind _asbp_snake_controller (cast `/Game/Snake/Character/BP_SnakeController` _returnvalue))
  (set `self.As BP Snake Controller` _asbp_snake_controller)
  (if (== (`GameplayStatics.GetPlayerControllerID` (`PlayerState.GetPlayerController` (`Controller.PlayerState` _returnvalue))) 0)
    (bind _assnake_game_instance (cast `SnakeGameInstance` (`GameplayStatics.GetGameInstance`)))
    (bind _returnvalue_2 (`SnakeGameInstance.GetSnakePlayerData` _assnake_game_instance 1))
    (`/Game/Snake/Character/BP_SnakeController.ShowOutro` (`self.As BP Snake Controller`) 2 (break `PlayerPersistentData` _returnvalue_2))
    (else
      (bind _assnake_game_instance_2 (cast `SnakeGameInstance` (`GameplayStatics.GetGameInstance`)))
      (bind _returnvalue_3 (`SnakeGameInstance.GetSnakePlayerData` _assnake_game_instance_2 0))
      (`/Game/Snake/Character/BP_SnakeController.ShowOutro` (`self.As BP Snake Controller`) 1 (break `PlayerPersistentData` _returnvalue_3)))))

(fn `UserConstructionScript`)