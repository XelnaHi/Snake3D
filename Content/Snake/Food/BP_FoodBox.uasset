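; BP_FoodBox is the food pickup in the Snake game, consumed when a BP_SnakeCharacter_New overlaps it.
; The overlap raises the snake's move speed, grows its tail and updates the score on its BP_SnakeState, passing the player controller ID.
; It then spawns a SimpleExplosion effect at its location and destroys itself.
; CheckIfFood always returns true, identifying the actor as food.
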(event `self.ReceiveActorBeginOverlap`
  (params (OtherActor :type "Actor Object Reference"))
  (bind _asbp_snake_character_new (cast `/Game/Snake/Character/BP_SnakeCharacter_New` OtherActor))
  (`SnakeCharacter.IncreaseMoveSpeed` _asbp_snake_character_new 1.5)
  (`SnakeCharacter.GrowTail` _asbp_snake_character_new)
  (bind _asbp_snake_state (cast `/Game/Snake/Character/BP_SnakeState` (`Pawn.PlayerState` _asbp_snake_character_new)))
  (`/Game/Snake/Character/BP_SnakeState.UpdateScore` _asbp_snake_state (`GameplayStatics.GetPlayerControllerID` (`PlayerState.GetPlayerController` (`Controller.PlayerState` (`Pawn.GetController` _asbp_snake_character_new)))))
  (`NiagaraFunctionLibrary.SpawnSystemAtLocation` "/Niagara/DefaultAssets/Templates/Systems/SimpleExplosion.SimpleExplosion" (`self.K2_GetActorLocation`))
  (`self.K2_DestroyActor`))

(fn `CheckIfFood`
  (returns (IsFood :type Boolean))
  (return true))

(fn `UserConstructionScript`)